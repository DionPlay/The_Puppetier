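; BP_CoffeeMachine is an interactible machine that brews a cup of coffee for the player character, BP_Dion2D, to pick up.
; Interact starts brewing when idle and empty, which shows the cup, plays a grinder sound and marks it full after a delay.
; Interacting with a full cup collects it unless the player's hands are full, setting the player's cup state and type.
; Tick syncs coffee visibility to the full flag.
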(event `self.ReceiveTick`
  (params (DeltaSeconds :type "Float (single-precision)"))
  (if (`self.IsCupFull`)
    (`SceneComponent.SetVisibility` (`self.Coffee`) true false)
    (else
      (`SceneComponent.SetVisibility` (`self.Coffee`) false false))))

(event `CollectCup`
  (`SceneComponent.SetVisibility` (`self.cup`) false false)
  (`SceneComponent.SetVisibility` (`self.cupsphere`) false false)
  (`GameplayStatics.PlaySoundAtLocation` "/Game/_Game/Audio/CollectCup_Cue.CollectCup_Cue" (`self.K2_GetActorLocation`) (struct) 1.0 1.0 0.0 null null null null)
  (`KismetSystemLibrary.PrintString` "cup collected")
  (set `self.IsCupFull` false)
  (bind _asbp_dion_2d (cast `/Game/_Game/2D/BP_Dion2D` (`GameplayStatics.GetPlayerCharacter` 0)))
  (set `/Game/_Game/2D/BP_Dion2D.hasCup` true _asbp_dion_2d)
  (set `/Game/_Game/2D/BP_Dion2D.cupType` "c" _asbp_dion_2d)
  (`SceneComponent.SetVisibility` (`self.Coffee`) false false))

(event `Turn On`
  (if (not (`self.IsOn`))
    (set `self.IsOn` true)
    (`SceneComponent.SetVisibility` (`self.cup`) true false)
    (`SceneComponent.SetVisibility` (`self.cupsphere`) true false)
    (`GameplayStatics.PlaySoundAtLocation` "/Game/_Game/Audio/CoffeeGrinder_Cue.CoffeeGrinder_Cue" (`self.K2_GetActorLocation`) (struct) 1.0 1.0 0.0 null null null null)
    (`KismetSystemLibrary.Delay` 7.0)
    (`KismetSystemLibrary.PrintString` "cup ready")
    (set `self.IsCupFull` true)
    (set `self.IsOn` false)))

(event `/Game/_Game/InteractionSystem/BPI_Interactible.Interact`
  (if (`self.IsOn`)
    (if (`self.IsCupFull`) :!label _label
      (bind _asbp_dion_2d (cast `/Game/_Game/2D/BP_Dion2D` (`GameplayStatics.GetPlayerCharacter` 0)))
      (if (`/Game/_Game/2D/BP_Dion2D.hasCup` _asbp_dion_2d)
        (`KismetSystemLibrary.PrintString` "Hands full")
        (else
          (`self.CollectCup`)))
      (else
        (`KismetSystemLibrary.PrintString` "wait")))
    (elif (`self.IsCupFull`)
      (goto _label)
      (else
        (`self.Turn On`)
        (`KismetSystemLibrary.PrintString` "on")))))

(fn `UserConstructionScript`)