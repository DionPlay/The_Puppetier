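; BP_TeaPot is an interactible that brews a cup of tea for the player to collect.
; Interact starts brewing when idle and empty, which shows the cup, plays a grinder sound and fills it after a fixed delay.
; Further interaction prints "wait" until the cup is full, then hands it to the player character as tea unless their hands are full.
; IsOn and IsCupFull track the state, with print-string feedback.
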(event `self.ReceiveBeginPlay`
  (`SceneComponent.SetVisibility` (`self.tea`) false false))

(event `CollectCup`
  (`SceneComponent.SetVisibility` (`self.cup`) false false)
  (`SceneComponent.SetVisibility` (`self.cupsphere`) false false)
  (`GameplayStatics.PlaySoundAtLocation` "/Game/_Game/Audio/CollectCup_Cue.CollectCup_Cue" (`self.K2_GetActorLocation`) (struct) 1.0 1.0 0.0 null null null null)
  (`KismetSystemLibrary.PrintString` "cup collected")
  (set `self.IsCupFull` false)
  (bind _asbp_third_person_character (cast `/Game/ThirdPerson/Blueprints/BP_ThirdPersonCharacter` (`GameplayStatics.GetPlayerCharacter` 0)))
  (set `/Game/ThirdPerson/Blueprints/BP_ThirdPersonCharacter.hasCup` true _asbp_third_person_character)
  (set `/Game/ThirdPerson/Blueprints/BP_ThirdPersonCharacter.cupType` "t" _asbp_third_person_character)
  (`SceneComponent.SetVisibility` (`self.tea`) false false))

(event `Turn On`
  (if (not (`self.IsOn`))
    (set `self.IsOn` true)
    (`SceneComponent.SetVisibility` (`self.cup`) true false)
    (`SceneComponent.SetVisibility` (`self.cupsphere`) true false)
    (`GameplayStatics.PlaySoundAtLocation` "/Game/_Game/Audio/CoffeeGrinder_Cue.CoffeeGrinder_Cue" (`self.K2_GetActorLocation`) (struct) 1.0 1.0 0.0 null null null null)
    (`KismetSystemLibrary.Delay` 7.0)
    (`KismetSystemLibrary.PrintString` "cup ready")
    (set `self.IsCupFull` true)
    (`SceneComponent.SetVisibility` (`self.tea`) true false)
    (set `self.IsOn` false)))

(event `self.Interact`
  (if (`self.IsOn`)
    (if (`self.IsCupFull`) :!label _label
      (bind _asbp_third_person_character (cast `/Game/ThirdPerson/Blueprints/BP_ThirdPersonCharacter` (`GameplayStatics.GetPlayerCharacter` 0)))
      (if (`/Game/ThirdPerson/Blueprints/BP_ThirdPersonCharacter.hasCup` _asbp_third_person_character)
        (`KismetSystemLibrary.PrintString` "Hands full")
        (else
          (`self.CollectCup`)))
      (else
        (`KismetSystemLibrary.PrintString` "wait")))
    (elif (`self.IsCupFull`)
      (goto _label)
      (else
        (`self.Turn On`)
        (`KismetSystemLibrary.PrintString` "on")))))

(fn `UserConstructionScript`)