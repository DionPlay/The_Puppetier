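; BP_NPC is an interactable customer that orders a random drink from the player character's menu and waits to be served.
; After a short delay on BeginPlay it picks the order and shows either its Coffee or Tea component.
; On Interact, a held cup of the matching type makes it face the player, play a coin sound, take the cup and destroy itself shortly afterwards.
; Otherwise it prints feedback to screen.
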(event `self.ReceiveBeginPlay`
  (set `self.isGiven` false)
  (`KismetSystemLibrary.Delay` 3.0)
  (bind _asbp_third_person_character (cast `/Game/ThirdPerson/Blueprints/BP_ThirdPersonCharacter` (`GameplayStatics.GetPlayerCharacter` 0)))
  (bind _output_get (set `self.isWanted` (`KismetArrayLibrary.Array_Random` (`/Game/ThirdPerson/Blueprints/BP_ThirdPersonCharacter.Menu` _asbp_third_person_character))))
  (if (`KismetStringLibrary.EqualEqual_StrStr` _output_get "c")
    (`SceneComponent.SetVisibility` (`self.Coffee`) true false)
    (else
      (`SceneComponent.SetVisibility` (`self.Tea`) true false))))

(event `/Game/_Game/InteractionSystem/BPI_Interactible.Interact`
  (if (not (`self.isGiven`))
    (`KismetSystemLibrary.PrintString` (`self.isWanted`))
    (bind _asbp_third_person_character (cast `/Game/ThirdPerson/Blueprints/BP_ThirdPersonCharacter` (`GameplayStatics.GetPlayerCharacter` 0)))
    (if (`/Game/ThirdPerson/Blueprints/BP_ThirdPersonCharacter.hasCup` _asbp_third_person_character)
      (if (`KismetStringLibrary.EqualEqual_StrStr` (`/Game/ThirdPerson/Blueprints/BP_ThirdPersonCharacter.cupType` _asbp_third_person_character) (stale `self.ReceiveBeginPlay` _output_get))
        (bind _asbp_third_person_character_2 (cast `/Game/ThirdPerson/Blueprints/BP_ThirdPersonCharacter` (`GameplayStatics.GetPlayerPawn` 0)))
        (`self.K2_SetActorRotation` (`KismetMathLibrary.FindLookAtRotation` (`self.K2_GetActorLocation`) (`self.K2_GetActorLocation` _asbp_third_person_character_2)))
        (`GameplayStatics.PlaySoundAtLocation` "/Game/_Game/Audio/CoinCollect_Cue.CoinCollect_Cue" (`self.K2_GetActorLocation`) (struct) 1.0 1.0 0.0 null null null null)
        (set `/Game/ThirdPerson/Blueprints/BP_ThirdPersonCharacter.hasCup` false _asbp_third_person_character)
        (set `self.isGiven` true)
        (`KismetSystemLibrary.Delay` 2.0)
        (`self.K2_DestroyActor`)
        (else
          (`KismetSystemLibrary.PrintString` "wrong cup")))
      (else
        (`KismetSystemLibrary.PrintString` "please give me my drink")))))

(fn `UserConstructionScript`)