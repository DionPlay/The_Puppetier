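; BP_NPCSpawner spawns BP_NPC actors at its Box component's location and starts them following waypoints.
; Tick drives the spawning through a random Delay of under ten seconds, incrementing NPCCounter after each spawn.
; Once the counter reaches three, spawning pauses until the most recently spawned NPC's IsGiven flag is true, which decrements the counter.
; Only that last NPC reference is stored and checked.
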(event `self.ReceiveTick`
  (params (DeltaSeconds :type "Float (single-precision)"))
  (if (== (`self.NPC_Counter`) 3)
    (if (`/Game/_Game/Interactibles/BP_NPC.isGiven` (stale _returnvalue))
      (set `self.NPC_Counter` (- (`self.NPC_Counter`) 1)))
    (else
      (`KismetSystemLibrary.Delay` (`KismetMathLibrary.Conv_IntToDouble` (`KismetMathLibrary.RandomInteger` 10)))
      (bind _returnvalue (`|SpawnActorFromClass` :`Class` "/Game/_Game/Interactibles/BP_NPC.BP_NPC_C" :`SpawnTransform` (`KismetMathLibrary.Conv_VectorToTransform` (`SceneComponent.GetSocketLocation` (`self.Box`) "None")) :`CollisionHandlingOverride` "Undefined" :`TransformScaleMethod` "MultiplyWithRoot" :`Instigator` null))
      (set `self.NPC_Counter` (+ (`self.NPC_Counter`) 1))
      (`/Game/_Game/Interactibles/BP_NPC.Follow Waypoints` _returnvalue))))

(fn `UserConstructionScript`)